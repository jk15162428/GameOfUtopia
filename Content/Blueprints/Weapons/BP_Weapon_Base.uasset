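; Base weapon Blueprint that fires a hitscan shot to score points on enemy targets.
; FireEvent line traces on the Visibility channel from the player camera along its forward vector, out to WeaponRange.
; A hit on a ScoreTarget flagged IsEnemy increments the PlayerCharacter's Score and plays the pistol fire sound, which is silent on any other shot.
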(event Custom|FireEvent
  (bind _returnvalue (Game|GetPlayerCameraManager 0))
  (bind _returnvalue_2 (Camera|GetCameraLocation _returnvalue))
  (bind (_outhit _returnvalue_3) (Collision|LineTraceByChannel _returnvalue_2 (+ _returnvalue_2 (* (Transformation|GetActorForwardVector _returnvalue) (Variables|Default|GetWeaponRange))) "TraceTypeQuery1" false 0 "None"))
  (if _returnvalue_3
    (bind _asscore_target (Utilities|Casting|CastToScoreTarget (.HitActor (Collision|BreakHitResult _outhit))))
    (if (Variables|/Game/Blueprints/Objects/ScoreTarget.ScoreTarget_C|GetIsEnemy _asscore_target)
      (bind _asplayer_character (Utilities|Casting|CastToPlayerCharacter (Game|Player|GetPlayerPawn 0)))
      (Variables|/Game/Blueprints/Characters/PlayerCharacter.PlayerCharacter_C|SetScore _asplayer_character (+ (Variables|/Game/Blueprints/Characters/PlayerCharacter.PlayerCharacter_C|GetScore _asplayer_character) 1))
      (Audio|PlaySound2D "/Game/Weapons/MilitaryWeapDark/Sound/Pistol/Wavs/PistolB_Fire01.PistolB_Fire01" 1.0 1.0 0.0 0 0))))

(event EventBeginPlay)

(event Collision|EventActorBeginOverlap
  (params (OtherActor :type Actor%20Object%20Reference)))

(event EventTick
  (params (DeltaSeconds :type Float%20%28single-precision%29)))

(fn ConstructionScript)